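; Canvas HUD for the main menu and multiplayer lobby, with hit-box buttons to host, join by IP, start or quit.
; Number, period and delete keys edit the IP string; button releases run console open or server-open commands, though Quit's command is empty.
; DrawButton pairs texture and label with a named hit box.
; DrawHUD is empty and main menu drawing is disconnected; lobby drawing sits in ReceiveDrawHUD_Copy, showing Start only on the server.
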(event `self.ReceiveDrawHUD`
  (params (SizeX :type Integer) (SizeY :type Integer))
  ;[1 1 1] Draw Main Menu
)

(event `Key|One`
  (params (Key :type "Key Structure" :default "AnyKey"))
  ;[1 1 1] Input for  IP Address
  (:`Released`
    (`self.BuildHostString` "1" :!label _label)))

(event `Key|Two`
  (params (Key :type "Key Structure" :default "AnyKey"))
  ;[1 1 1] Input for  IP Address
  (:`Released`
    (`self.BuildHostString` "2" :!label _label_2)))

(event `Key|Three`
  (params (Key :type "Key Structure" :default "AnyKey"))
  ;[1 1 1] Input for  IP Address
  (:`Released`
    (`self.BuildHostString` "3" :!label _label_3)))

(event `Key|NumPadOne`
  (params (Key :type "Key Structure" :default "AnyKey"))
  ;[1 1 1] Input for  IP Address
  (:`Released`
    (goto _label)))

(event `Key|NumPadTwo`
  (params (Key :type "Key Structure" :default "AnyKey"))
  ;[1 1 1] Input for  IP Address
  (:`Released`
    (goto _label_2)))

(event `Key|NumPadThree`
  (params (Key :type "Key Structure" :default "AnyKey"))
  ;[1 1 1] Input for  IP Address
  (:`Released`
    (goto _label_3)))

(event `Key|Four`
  (params (Key :type "Key Structure" :default "AnyKey"))
  ;[1 1 1] Input for  IP Address
  (:`Released`
    (`self.BuildHostString` "4" :!label _label_4)))

(event `Key|Five`
  (params (Key :type "Key Structure" :default "AnyKey"))
  ;[1 1 1] Input for  IP Address
  (:`Released`
    (`self.BuildHostString` "5" :!label _label_5)))

(event `Key|Six`
  (params (Key :type "Key Structure" :default "AnyKey"))
  ;[1 1 1] Input for  IP Address
  (:`Released`
    (`self.BuildHostString` "6" :!label _label_6)))

(event `Key|NumPadFour`
  (params (Key :type "Key Structure" :default "AnyKey"))
  ;[1 1 1] Input for  IP Address
  (:`Released`
    (goto _label_4)))

(event `Key|NumPadFive`
  (params (Key :type "Key Structure" :default "AnyKey"))
  ;[1 1 1] Input for  IP Address
  (:`Released`
    (goto _label_5)))

(event `Key|NumPadSix`
  (params (Key :type "Key Structure" :default "AnyKey"))
  ;[1 1 1] Input for  IP Address
  (:`Released`
    (goto _label_6)))

(event `Key|Eight`
  (params (Key :type "Key Structure" :default "AnyKey"))
  ;[1 1 1] Input for  IP Address
  (:`Released`
    (`self.BuildHostString` "8" :!label _label_7)))

(event `Key|Nine`
  (params (Key :type "Key Structure" :default "AnyKey"))
  ;[1 1 1] Input for  IP Address
  (:`Released`
    (`self.BuildHostString` "9" :!label _label_8)))

(event `Key|Seven`
  (params (Key :type "Key Structure" :default "AnyKey"))
  ;[1 1 1] Input for  IP Address
  (:`Released`
    (`self.BuildHostString` "7" :!label _label_9)))

(event `Key|NumPadNine`
  (params (Key :type "Key Structure" :default "AnyKey"))
  ;[1 1 1] Input for  IP Address
  (:`Released`
    (goto _label_8)))

(event `Key|NumPadSeven`
  (params (Key :type "Key Structure" :default "AnyKey"))
  ;[1 1 1] Input for  IP Address
  (:`Released`
    (goto _label_9)))

(event `Key|NumPadEight`
  (params (Key :type "Key Structure" :default "AnyKey"))
  ;[1 1 1] Input for  IP Address
  (:`Released`
    (goto _label_7)))

(event `Key|Decimal`
  (params (Key :type "Key Structure" :default "AnyKey"))
  ;[1 1 1] Input for  IP Address
  (:`Released`
    (`self.BuildHostString` "." :!label _label_10)))

(event `Key|BackSpace`
  (params (Key :type "Key Structure" :default "AnyKey"))
  ;[1 1 1] Input for  IP Address
  (:`Released`
    (`self.DeleteStringCharacter` :!label _label_11)))

(event `Key|Zero`
  (params (Key :type "Key Structure" :default "AnyKey"))
  ;[1 1 1] Input for  IP Address
  (:`Released`
    (`self.BuildHostString` "0" :!label _label_12)))

(event `Key|Delete`
  (params (Key :type "Key Structure" :default "AnyKey"))
  ;[1 1 1] Input for  IP Address
  (:`Released`
    (goto _label_11)))

(event `Key|Period`
  (params (Key :type "Key Structure" :default "AnyKey"))
  ;[1 1 1] Input for  IP Address
  (:`Released`
    (goto _label_10)))

(event `Key|NumPadZero`
  (params (Key :type "Key Structure" :default "AnyKey"))
  ;[1 1 1] Input for  IP Address
  (:`Released`
    (goto _label_12)))

(event `ReceiveDrawHUD_Copy`
  (params (SizeX :type Integer) (SizeY :type Integer))
  (bind _buttontexture (`self.ButtonTexture`))
  (bind (_x _y) (`KismetMathLibrary.BreakVector2D` (`self.ScreenDimensions`)))
  ;[1 1 1] Draw Lobby Menu
  ;;[1 1 1] Setup Button and Screen Sizes
  (set `self.ButtonSize` (`KismetMathLibrary.MakeVector2D` (`KismetMathLibrary.Conv_IntToDouble` (`Texture2D.Blueprint_GetSizeX` _buttontexture)) (`KismetMathLibrary.Conv_IntToDouble` (`Texture2D.Blueprint_GetSizeY` _buttontexture))))
  (set `self.ScreenDimensions` (`KismetMathLibrary.MakeVector2D` (`KismetMathLibrary.Conv_IntToDouble` SizeX) (`KismetMathLibrary.Conv_IntToDouble` SizeY)))
  ;;[1 1 1] Lobby Menu Conditional
  (if (`self.LobbyIsActive`)
    ;;[1 1 1] Draw Background
    (`self.DrawMaterialSimple` null 0.0 0.0 _x _y)
    (if (`KismetSystemLibrary.IsServer`)
      ;;[1 1 1] Draw Start Button
      (`self.DrawButton` (`KismetMathLibrary.MakeVector2D` 10.0 200.0) (`self.ButtonSize`) "Start" (select `bool` (`self.StartButtonPressed`) :`false` (`self.ButtonTexture`) :`true` (`self.ButtonTexturePressed`)) (`self.TextColor`)))
    ;;[1 1 1] Draw Quit Button
    (`self.DrawButton` (`KismetMathLibrary.MakeVector2D` 10.0 400.0) (`self.ButtonSize`) "Quit" (select `bool` (`self.HostButtonPressed`) :`false` (`self.ButtonTexture`) :`true` (`self.ButtonTexturePressed`)) (`self.TextColor`))))

(event `self.ReceiveHitBoxClick`
  (params (BoxName :type Name))
  ;[1 1 1] On Click Events
  (switch `name` BoxName
    (:`Host`
      (set `self.HostButtonPressed` true))
    (:`Join`
      (set `self.JoinButtonPressed` true))
    (:`Quit`
      (set `self.QuitButtonPressed` true))
    (:`Start`
      (set `self.StartButtonPressed` true))))

(event `self.ReceiveHitBoxRelease`
  (params (BoxName :type Name))
  ;[1 1 1] On Click Events
  (switch `name` BoxName
    (:`Host`
      (`KismetSystemLibrary.ExecuteConsoleCommand` (`KismetStringLibrary.Concat_StrStr` "Open " "Lobby?Listen")))
    (:`Join`
      (`KismetSystemLibrary.ExecuteConsoleCommand` (`KismetStringLibrary.Concat_StrStr` "Open " (`self.ipString`))))
    (:`Quit`
      (`KismetSystemLibrary.ExecuteConsoleCommand` ""))
    (:`Start`
      (set `self.LobbyIsActive` false)
      (set `self.MainMenuIsActive` false)
      (`KismetSystemLibrary.ExecuteConsoleCommand` (`KismetStringLibrary.Concat_StrStr` "ServerOpen" (`self.GameLevelName`))))))

(event `Key|LeftMouseButton`
  (params (Key :type "Key Structure" :default "AnyKey"))
  ;[1 1 1] On Click Events
  (:`Released`
    (set `self.HostButtonPressed` false)
    (set `self.JoinButtonPressed` false)
    (set `self.QuitButtonPressed` false)
    (set `self.StartButtonPressed` false)))

(fn `BuildHostString`
  (params (`Key Input` :type String))
  (set `self.ipString` (`KismetStringLibrary.Concat_StrStr` (`self.ipString`) `Key Input`)))

(fn `DeleteStringCharacter`
  (bind _ipstring (`self.ipString`))
  (set `self.ipString` (`KismetStringLibrary.GetSubstring` _ipstring 0 (- (`KismetStringLibrary.Len` _ipstring) 1))))

(fn `DrawButton`
  (params (ButtonScreenLocation :type "Vector2D Structure") (ButtonSize :type "Vector2D Structure") (ButtonText :type String) (ButtonTexture :type "Texture2D Object Reference") (TextColor :type "LinearColor Structure"))
  (bind (_x _y) (`KismetMathLibrary.BreakVector2D` ButtonScreenLocation))
  (bind (_outwidth _outheight) (`self.GetTextSize` ButtonText))
  (bind (_x_2 _y_2) (`KismetMathLibrary.BreakVector2D` (- (+ (/ ButtonSize 2.0) ButtonScreenLocation) (/ (`KismetMathLibrary.MakeVector2D` _outwidth _outheight) 1.0))))
  ;[1 1 1] Draw Button
  (`self.DrawTextureSimple` ButtonTexture _x _y)
  ;[1 1 1] Draw Text On Button
  (`self.DrawText` ButtonText TextColor _x_2 _y_2 null 2.0)
  ;[1 1 1] Add Hit Box To Button
  (`self.AddHitBox` ButtonScreenLocation ButtonSize (`KismetStringLibrary.Conv_StringToName` ButtonText)))

(fn `UserConstructionScript`)